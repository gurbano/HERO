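; Hero character Blueprint that extends a parent locomotion character with physical animation, combat and widget components.
; BeginPlay initializes the components, caches the hero AnimInstance and forwards ragdoll state changes to the physics component.
; Overrides roll and get-up montages for one-handed weapon and combat overlay states, otherwise deferring to the parent.
; A timeline eases yaw toward a given enemy; input keys trigger attack and debug physical animation or hit reactions.
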(event `self.ReceiveActorBeginOverlap`
  (params (OtherActor :type "Actor Object Reference"))
  (`KismetSystemLibrary.PrintString` "Hello")
  (cast `/Game/BP_Target` OtherActor))

(event `self.ReceiveTick`
  (params (DeltaSeconds :type "Float (single-precision)")))

(event `RotateToEnemy`
  (params (Enemy :type "Actor Object Reference"))
  (bind (_returnvalue_roll _returnvalue_pitch _returnvalue_yaw) (`KismetMathLibrary.BreakRotator` (`KismetMathLibrary.FindLookAtRotation` (`self.K2_GetActorLocation`) (`self.K2_GetActorLocation` Enemy))))
  ;[1 1 1 1 40] ROTATE TO ENEMY EVENT
  (`/Engine/EditorBlueprintResources/StandardMacros.IsValid` Enemy
    (:`Is Valid`
      (`Timeline|RotateTooEnemyTimeline` :!via `PlayFromStart`
        (:`Update`
          (`self.K2_SetActorRotation` (`KismetMathLibrary.RInterpTo` (`self.K2_GetActorRotation`) (`KismetMathLibrary.MakeRotator` 0.0 0.0 _returnvalue_yaw) 0.1 1.0)))
        (:`Finished`)))))

(event `OnRagdollChanged` :!signature `self.RagdollStateChangedDelegate`
  (params (bRagdollState :type Boolean))
  ;[1 1 1 1 70] INIT
  ;;[1 1 1] INIT BCP_PHY
  (`/Game/BPC/BPC_Phy.OnRagdollChangeState` (`self.BPC_Phy`) bRagdollState))

(event `self.ReceiveBeginPlay`
  (bind _bpc_phy (`self.BPC_Phy`))
  ;[1 1 1 1 70] INIT
  (`|ExecutionSequence`
    (:`then_0`
      ;;[1 1 1] INIT BCP_PHY
      (`/Game/BPC/BPC_Phy.InitFunction` _bpc_phy)
      (`/Game/BPC/BPC_Phy.TogglePhysicalAnim` _bpc_phy false)
      (add `self.RagdollStateChangedDelegate` (delegate `OnRagdollChanged`)))
    (:`then_1`
      ;;[1 1 1] INIT BPC COMBAT
      (`/Game/BPC/BPC_Combat.Init Function` (`self.BPC_Combat`))
      ;;[1 1 1] Init REF TO ABP_HERO
      (bind _asabp_hero (cast `/Game/ABP_Hero` (`SkeletalMeshComponent.GetAnimInstance` (`self.Mesh`))))
      (set `self.Anim Instance` _asabp_hero))
    (:`then_2`
      (`/Game/BPC/BPC_Widgets.Init` (`self.BPC_Widgets`) (`self.CombatStateWidget`)))))

(event `Key|Zero`
  (params (Key :type "Key Structure"))
  (bind _bpc_phy (`self.BPC_Phy`))
  ;[1 1 1 1 100] DEBUG
  (:`Pressed`
    (`/Game/BPC/BPC_Phy.TogglePhysicalAnim` _bpc_phy (not (`/Game/BPC/BPC_Phy.isSimulating` _bpc_phy)))))

(event `Key|BackSpace`
  (params (Key :type "Key Structure"))
  ;[1 1 1 1 100] DEBUG
  (:`Pressed`
    (`/Game/BPC/BPC_Phy.HitReaction` :`self` (`self.BPC_Phy`))))

(event `Key|LeftMouseButton`
  (params (Key :type "Key Structure"))
  ;[1 1 1 1 100] DEBUG
  (:`Pressed`
    (`/Game/BPC/BPC_Combat.PlayAttackONE` (`self.BPC_Combat`))))

(fn `GetGetUpAnimation`
  (params (bRagdollFaceUpState :type Boolean))
  (returns (ReturnValue :type "AnimMontage Object Reference"))
  (locals (NewLocalVar_0 :type "AnimMontage Object Reference"))
  (bind _returnvalue (`self.IsCustomState`))
  (if _returnvalue
    (if bRagdollFaceUpState
      (return "/Game/Combat/Montages/JumpUpMontage.JumpUpMontage")
      (else
        (return (`self.GetUpFront_LH`))))
    (else
      (bind _returnvalue_2 (`parent.GetGetUpAnimation` bRagdollFaceUpState))
      (return _returnvalue_2))))

(fn `GetRollAnimation`
  (returns (ReturnValue :type "AnimMontage Object Reference"))
  (bind _returnvalue (`self.IsCustomState`))
  (if _returnvalue
    (return (`self.LandRoll_2H`))
    (else
      (bind _returnvalue_2 (`parent.GetRollAnimation`))
      (return _returnvalue_2))))

(fn `IsCustomState`
  (returns (ReturnValue :type Boolean))
  (bind _overlaystate (`self.OverlayState`))
  (return (or (`|EnumEquality` _overlaystate "Weapon1H") (`|EnumEquality` _overlaystate "Combat"))))

(fn `UserConstructionScript`
  (`parent.UserConstructionScript`))
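; BP_AttackBase is a base for attacks, holding a range, a knockout chance, a KO type and a KO montage.
; Init assigns a new UUID, and IsInRange compares a given distance against the range.
; ComputeKOChance scales KO chance by hit bone, boosting head, neck and clavicles and zeroing arms and hands.
; Its hit direction and attacker and defender location inputs are unused.
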(fn `ComputeKOChance`
  (params (HitBone :type Name) (HitDirection :type "Vector Structure") (AttackerLocation :type "Vector Structure") (DefenderLocation :type "Vector Structure"))
  (returns (KOChance :type "Float (double-precision)") (KOType :type "/Game/BPC/AttackBase/E_KOType Enum") (KOMontage :type "AnimMontage Object Reference"))
  (locals (p_HitBone :type Name) (p_BoneMult :type "Float (double-precision)" :default 1.0))
  (bind _output_get (set `local.p_HitBone` HitBone))
  (switch `name` _output_get
    (:`Default`
      (set `local.p_BoneMult` 1.0))
    (:`Head`
      (set `local.p_BoneMult` 5.0 :!label _label))
    (:`neck_01`
      (goto _label))
    (:`UpperArm_L`
      (set `local.p_BoneMult` 0.0 :!label _label_2))
    (:`UpperArm_R`
      (goto _label_2))
    (:`clavicle_l`
      (set `local.p_BoneMult` 2.0 :!label _label_3))
    (:`clavicle_r`
      (goto _label_3))
    (:`lowerarm_l`
      (goto _label_2))
    (:`lowerarm_r`
      (goto _label_2))
    (:`Hand_L`
      (goto _label_2))
    (:`Hand_R`
      (goto _label_2)))
  (return (* (`self.KOChance`) (`local.p_BoneMult`)) (`self.KOType`) (`self.KOMontage`)))

(fn `Init`
  (set `self.UUID` (`KismetGuidLibrary.NewGuid`))
  (return))

(fn `isInRange`
  (params (Distance :type "Float (double-precision)"))
  (returns (InRange :type Boolean))
  (return (<= Distance (`self.Range`))))
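; BPC_Combat is BP_Hero's melee component, handling both attacking and defending.
; An attack picks a random attack object, alerts and faces the target, then plays its montage with optional slow motion.
; Anim-notify-toggled sphere traces on hand, head or foot sockets pass hits to the target's component.
; The defender guards after a random delay, then resolves arm blocks, chance-based KOs or hit reactions via BPCPhy, reporting non-KO results back.
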(event `PerformAttackAction`
  (params (Enemy :type "/Game/BP_Hero Object Reference"))
  (bind _currentattack (`self.CurrentAttack`))
  (bind _montage (`/Game/BPC/AttackBase/BP_AttackBase.Montage` _currentattack))
  ;[1 0.2528 0.1129 1 60] PERFORM ATTACK
  ;;[1 1 1 1 25] CanAttack
  (if (not (`/Game/BPC/BPC_Combat.isAttacking` (`/Game/BP_Hero.BPC_Combat` (`self.As BP Hero`))))
    ;;[1 1 1 1 25] Find enemy if not set
    (`/Engine/EditorBlueprintResources/StandardMacros.IsValid` Enemy
      (:`Is Valid`
        (set `self.Enemy` Enemy))
      (:`Is Not Valid`
        (bind _asbp_hero (`self.FindNearestTarget`))
        (set `self.Enemy` _asbp_hero)))
    ;;[1 1 1 1 25] SELECT ATTACK
    (bind _attack (`self.Select Attack`))
    (set `self.CurrentAttack` _attack)
    ;;[1 1 1 1 25] NOTIFY ENEMY
    (`self.Targeted` (`/Game/BP_Hero.BPC_Combat` (`self.Enemy`)) self (`self.CurrentAttack`))
    ;;[1 1 1 1 25] ROTATE/MOVE
    (`/Game/BP_Hero.RotateToEnemy` (`self.As BP Hero`) (`self.Enemy`))
    ;;[1 1 1 1 25] SLOMO ON
    (if (`self.SlomoAttack`)
      (`self.Toggle Slomo`))
    ;;[1 1 1 1 25] PLAY MONTAGE
    (`|PlayMontage` (`self.Mesh`) _montage (`/Game/BPC/AttackBase/BP_AttackBase.MontageSpeed` _currentattack) 0.0 "Default"
      (:`OnCompleted`
        _)
      (:`OnInterrupted`
        (`Character.StopAnimMontage` (`self.As BP Hero`) _montage)))
    ;;[1 1 1 1 25] SLOMO OFF
    (if (`self.SlomoAttack`)
      (`self.Toggle Slomo`))))

(event `self.ReceiveTick`
  (params (DeltaSeconds :type "Float (single-precision)"))
  ;[0.8625 1 0.1563 1 66] EVENT TICK
  (`|ExecutionSequence`
    (:`then_0`
      ;[1 1 1] 1. CALL PERFORM TRACE
      (if (`self.IsTraceOn`)
        (`self.PerformTrace`)))
    (:`then_1`
      ;[1 1 1] DEBUG ENEMY
      (bind _enemy (`self.Enemy`)
        (:`then`)
        (:`else`)))))

(event `self.ReceiveBeginPlay`)

(event `TraceOn`
  (params (Trace :type Boolean) (PartToTrace :type "/Game/E_TracedAttacks Enum" :default "NewEnumerator0"))
  ;[1 0.2528 0.1129 1 60] SET TRACE ON/OFF (triggered from anim notify)
  (bind _output_get (set `self.IsTraceOn` Trace))
  (set `self.PartToTrace` PartToTrace))

(event `PerformTrace`
  (bind _returnvalue (`SceneComponent.GetSocketLocation` (`Character.Mesh` (`self.As BP Hero`)) (select `/Game/E_TracedAttacks` (`self.PartToTrace`) :`NewEnumerator0` "middle_01_l" :`NewEnumerator1` "middle_01_r" :`NewEnumerator2` "Head" :`NewEnumerator3` "Foot_L" :`NewEnumerator4` "Foot_R" :!type "Name")))
  ;[1 0.2528 0.1129 1 60] PERFORM TRACE >> HIT REACTION
  (bind _outhits (`KismetSystemLibrary.SphereTraceMultiForObjects` _returnvalue _returnvalue 15.0 (`|MakeArray` "ObjectTypeQuery3" :!type "EObjectTypeQuery Enum") false (`|MakeArray` (`self.As BP Hero`) :!type "Actor Object Reference")))
  (for _array_element _outhits
    (`self.BeingHit` (`/Game/BP_Hero.BPC_Combat` (`self.Enemy`)) self _array_element (`self.CurrentAttack`))
    (break)))

(event `Targeted`
  (params (Attacker :type "/Game/BPC/BPC_Combat Object Reference") (Attack :type "/Game/BPC/AttackBase/BP_AttackBase Object Reference"))
  ;[0.8223 0.3229 1 1 44] BEING TARGETED (try to counter)
  (`KismetSystemLibrary.Delay` (`KismetMathLibrary.RandomFloatInRange` 0.0 0.3))
  (`KismetSystemLibrary.PrintString` "Paro")
  (if (not (`/Game/BPC/AttackBase/BP_AttackBase.processed` Attack))
    (set `/Game/ABP_Hero.GuardUp` true (`self.As ABP Hero`))
    (set `self.isBlocking` true)))

(event `Being Missed`
  ;[1 0.5137 0.7647 1 44] BEING MISSED (Called from IsAttackingState Anim Notify)
  (set `/Game/ABP_Hero.GuardUp` false (`self.As ABP Hero`)))

(event `BeingHit`
  (params (Attacker :type "/Game/BPC/BPC_Combat Object Reference") (HitResult :type "HitResult Structure") (Attack :type "/Game/BPC/AttackBase/BP_AttackBase Object Reference"))
  (bind _as_bp_hero (`self.As BP Hero`))
  ;[1 0.5137 0.7647] IF NOT PROCESSED
  (if (not (`/Game/BPC/AttackBase/BP_AttackBase.processed` Attack))
    ;[1 1 1] Rotate To Enemy
    (`/Game/BP_Hero.RotateToEnemy` _as_bp_hero (`self.GetOwner` Attacker))
    ;[1 1 1] IsValidBone
    (bind (_location _hitbonename _impulse) (`/Game/BPC/BPC_Phy.BreakHitResult` (`/Game/BP_Hero.BPC_Phy` _as_bp_hero) HitResult))
    (if (!= _hitbonename "None")
      (set `/Game/BPC/AttackBase/BP_AttackBase.HitBone` _hitbonename Attack)
      ;[1 1 1 1 40] Check IF Blocked
      (if (and (`self.isBlocking`) (`KismetArrayLibrary.Array_Contains` (`|MakeArray` "UpperArm_L" "UpperArm_R" "lowerarm_l" "lowerarm_r" "Hand_L" "Hand_R" :!type "Name") _hitbonename))
        ;[1 1 1 1 30] Update Attack
        (set `/Game/BPC/AttackBase/BP_AttackBase.blocked` true Attack)
        (set `/Game/BPC/AttackBase/BP_AttackBase.processed` true Attack)
        ;[1 1 1 1 30] Update State
        (set `self.isBlocking` false)
        (`self.AttackProcessed` Attacker Attack :!label _label)
        (set `/Game/ABP_Hero.GuardUp` false (`self.As ABP Hero`))
        (else
          (set `/Game/BPC/AttackBase/BP_AttackBase.processed` true Attack)
          (set `/Game/BPC/AttackBase/BP_AttackBase.hit` true Attack)
          ;[1 1 1 1 30] IF Check KO
          (bind (_isko _ko_type) (`self.CheckKO` Attack Attacker self _hitbonename _impulse))
          (if _isko
            (set `self.isKo` true)
            (set `self.isBlocking` false)
            ;[1 1 1] KO
            (`/Game/BPC/BPC_Phy.GoKO` (`/Game/BP_Hero.BPC_Phy` (`self.As BP Hero`)) _ko_type)
            (else
              (set `self.isBlocking` false)
              ;[1 1 1] Take Hit
              (`/Game/BPC/BPC_Phy.HitReaction` (`/Game/BP_Hero.BPC_Phy` (`self.As BP Hero`)) HitResult Attacker Attack)
              (goto _label))))))))

(fn `AttackProcessed`
  (params (Attack :type "/Game/BPC/AttackBase/BP_AttackBase Object Reference"))
  (locals (NewLocalVar_0 :type "/Game/BPC/AttackBase/BP_AttackBase Object Reference") (NewLocalVar_1 :type "/Game/BPC/AttackBase/BP_AttackBase Object Reference"))
  (bind _hitbone (`/Game/BPC/AttackBase/BP_AttackBase.HitBone` Attack))
  (bind _returnvalue (`KismetStringLibrary.Conv_NameToString` (`/Game/BPC/AttackBase/BP_AttackBase.Name` Attack)))
  (bind _returnvalue_2 (`KismetStringLibrary.Conv_NameToString` _hitbone))
  (if (`/Game/BPC/AttackBase/BP_AttackBase.hit` Attack)
    (`KismetSystemLibrary.PrintString` (`KismetStringLibrary.Concat_StrStr` (`KismetStringLibrary.Concat_StrStr` _returnvalue " - HIT - ") _returnvalue_2))
    (elif (`/Game/BPC/AttackBase/BP_AttackBase.blocked` Attack)
      (`AnimInstance.Montage_Stop` (`SkeletalMeshComponent.GetAnimInstance` (`self.Mesh`)) 0.3 (`/Game/BPC/AttackBase/BP_AttackBase.Montage` Attack))
      (`KismetSystemLibrary.PrintString` (`KismetStringLibrary.Concat_StrStr` (`KismetStringLibrary.Concat_StrStr` _returnvalue " - Blocked - ") _returnvalue_2))
      (elif (`/Game/BPC/AttackBase/BP_AttackBase.missed` Attack)
        (`KismetSystemLibrary.PrintString` (`KismetStringLibrary.Concat_StrStr` (`KismetStringLibrary.Concat_StrStr` _returnvalue " - MISSED - ") _returnvalue_2))
        (else
          (`KismetSystemLibrary.PrintString` (`KismetStringLibrary.Concat_StrStr` (`KismetStringLibrary.Concat_StrStr` _returnvalue " - ERROR - ") (`KismetStringLibrary.Conv_NameToString` _hitbone))))))))

(fn `CanAttack`
  ;[1 1 1] Not Attacking
  (if (not (`/Game/BPC/BPC_Combat.isAttacking` (`/Game/BP_Hero.BPC_Combat` (`self.As BP Hero`))))
    (return)))

(fn `CheckKO`
  (params (Attack :type "/Game/BPC/AttackBase/BP_AttackBase Object Reference") (Attacker :type "/Game/BPC/BPC_Combat Object Reference") (Target :type "/Game/BPC/BPC_Combat Object Reference") (HitBone :type Name) (HitDirection :type "Vector Structure"))
  (returns (IsKO :type Boolean) (`KO Type` :type "/Game/BPC/AttackBase/E_KOType Enum") (KOMontage :type "AnimMontage Object Reference"))
  (bind (_kochance _kotype _komontage) (`/Game/BPC/AttackBase/BP_AttackBase.ComputeKOChance` Attack HitBone HitDirection (`Actor.K2_GetActorLocation` (`self.GetOwner` Attacker)) (`Actor.K2_GetActorLocation` (`self.GetOwner` Target))))
  (return (< (`KismetMathLibrary.RandomFloatInRange` 0.0 100.0) _kochance) _kotype _komontage))

(fn `FindNearestTarget`
  (returns (AsBP_Hero :type "/Game/BP_Hero Object Reference"))
  (bind _outactors (`GameplayStatics.GetAllActorsOfClass` "/Game/BP_Target.BP_Target_C"))
  (bind _asbp_hero (cast `/Game/BP_Hero` (`.ReturnValue` (`GameplayStatics.FindNearestActor` (`Actor.K2_GetActorLocation` (`self.As BP Hero`)) _outactors))))
  (return _asbp_hero))

(fn `Init Function`
  (`|ExecutionSequence`
    (:`then_0`
      (bind _asbp_hero (cast `/Game/BP_Hero` (`self.GetOwner`)))
      (bind _output_get (set `self.As BP Hero` _asbp_hero))
      (bind _mesh (`Character.Mesh` _output_get))
      (set `self.Mesh` _mesh)
      (bind _asabp_hero (cast `/Game/ABP_Hero` (`SkeletalMeshComponent.GetAnimInstance` _mesh)))
      (set `self.As ABP Hero` _asabp_hero)
      (set `/Game/ABP_Hero.GuardUp` false _asabp_hero))
    (:`then_1`
      (for _array_element (`self.CombatAttackClasses`)
        (bind _returnvalue (`|GenericCreateObject` _array_element))
        (`KismetArrayLibrary.Array_Add` (`self.CombatAttacks`) _returnvalue)))))

(fn `PlayAttackONE`
  (`self.PerformAttackAction` null))

(fn `Select Attack`
  (returns (Attack :type "/Game/Combat/Attacks/BP_CombatAttack Object Reference"))
  (bind _returnvalue (`|GenericCreateObject` (`KismetArrayLibrary.Array_Random` (`self.CombatAttackClasses`))))
  (`/Game/BPC/AttackBase/BP_AttackBase.Init` _returnvalue)
  (return _returnvalue))

(fn `Toggle Slomo`
  (`ALSDebugComponent.ToggleSlomo` (`/ALSV4_CPP/AdvancedLocomotionV4/Blueprints/CharacterLogic/ALS_CharacterBP.DebugComponent` (`self.As BP Hero`)))
  (return))
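; BPC_Widgets is a component that feeds combat state into a combat state widget.
; Init takes a widget component, casts its user widget to CombatStateWidget and caches it.
; UpdateAttackState reads the owner's BPCCombat, setting the widget's current action to attack, block or empty, and copies the current attack.
; BeginPlay and Tick are empty, so neither function is driven from within this component.
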(event `self.ReceiveBeginPlay`)

(event `self.ReceiveTick`
  (params (DeltaSeconds :type "Float (single-precision)")))

(fn `Init`
  (params (CombatStateWidget :type "WidgetComponent Object Reference"))
  (bind _ascombat_state_widget (cast `/Game/BPC/Widgets/CombatStateWidget` (`WidgetComponent.GetUserWidgetObject` CombatStateWidget)))
  (set `self.As Combat State Widget` _ascombat_state_widget))

(fn `UpdateAttackState`
  (params (Owner :type "/Game/BP_Hero Object Reference"))
  (`|ExecutionSequence`
    (:`then_0`
      (if (`/Game/BPC/BPC_Combat.isAttacking` (`/Game/BP_Hero.BPC_Combat` Owner))
        (set `/Game/BPC/Widgets/CombatStateWidget.CurrentAction` "attack" (`self.As Combat State Widget`))
        (elif (`/Game/BPC/BPC_Combat.isBlocking` (`/Game/BP_Hero.BPC_Combat` Owner))
          (set `/Game/BPC/Widgets/CombatStateWidget.CurrentAction` "block" (`self.As Combat State Widget`))
          (else
            (set `/Game/BPC/Widgets/CombatStateWidget.CurrentAction` "" (`self.As Combat State Widget`))))))
    (:`then_1`
      (set `/Game/BPC/Widgets/CombatStateWidget.CurrentAttack` (`/Game/BPC/BPC_Combat.CurrentAttack` (`/Game/BP_Hero.BPC_Combat` Owner)) (`self.As Combat State Widget`)))))
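; Hero component that adds physical-animation hit reactions, stumbles and random knockouts to BP_Hero.
; HitReaction, triggered from BPC_COMBAT, simulates upper body and thighs under a "Strong" profile and applies a horizontal impulse against the impact normal.
; Tick decays a timer that drives upper-body physics blend weight and pushes movement along the impulse, then stops simulation.
; A KO chance roll triggers timed ragdoll, with optional slow motion.
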(event `TogglePhysicalAnim`
  (params (simulate :type Boolean))
  ;[0.4497 0.0588 1 1 50] TogglePhyAnim
  (`self.ToggleSimulation` simulate)
  (set `self.HitReactionTimeRemaining` 0.5)
  (`self.SetComponentTickEnabled` false))

(event `HitReaction`
  (params (hit :type "HitResult Structure") (Attacker :type "/Game/BPC/BPC_Combat Object Reference"))
  (bind _debugcomponent (`/ALSV4_CPP/AdvancedLocomotionV4/Blueprints/CharacterLogic/ALS_CharacterBP.DebugComponent` (`self.As BP Hero`)))
  ;[0.4497 0.0588 1 1 50] HitReaction Event (triggered in BPC_COMBAT)
  ;  TODO: MOVE DECISION LOGIC INTO BPC_COMBAT
  (bind (_location _hitbonename) (`self.BreakHitResult` hit))
  ;;[1 0.5664 0.7406 1 25] IF Not Simulating
  (if (not (`self.isSimulating`))
    ;;[1 1 1 1 25] IF Hit Some Bone
    (if (!= _hitbonename "None")
      ;;[1 1 1] TOGGLE SIMULATION
      (set `self.HitReactionTimeRemaining` (+ (`self.HitReactionTimeRemaining`) (`self.DefaultHitTimeRemaining`)))
      (`self.ToggleSimulation` true)
      (bind (_location_2 _hitbonename_2 _impulse _impactpoint _impactnormal) (`self.BreakHitResult` hit))
      ;;[1 1 1] Set Variables
      (set `self.HitLocation` _location_2)
      (set `self.LastImpulse` _impulse)
      (set `self.Hit Bone Name` _hitbonename_2)
      (set `self.LastImpactPoint` _impactpoint)
      (set `self.LastImpactNormal` _impactnormal)
      ;;[1 1 1] ADD IMPULSE
      (`PrimitiveComponent.AddImpulseAtLocation` (`self.Mesh`) (`self.LastImpulse`) (`self.HitLocation`) (`self.Hit Bone Name`))
      (`SkeletalMeshComponent.AddImpulseToAllBodiesBelow` (`self.Mesh`) (`self.LastImpulse`) (`self.Hit Bone Name`) false false)
      ;[1 1 1] KO - MOVE DECISION LOGIC
      (if (< (`KismetMathLibrary.RandomInteger` 100) (`self.KOChance`))
        (`|ExecutionSequence`
          (:`then_0`
            ;[1 1 1] SLOMO
            (if (`self.KOSlomo`)
              (`ALSDebugComponent.ToggleSlomo` _debugcomponent)
              (`KismetSystemLibrary.K2_SetTimer` _debugcomponent "ToggleSlomo" 0.2)))
          (:`then_1`
            ;[1 1 1] TODO: different KO for attack/hitbone
            (`self.TurnRagdollFor` 5.0)))))))

(event `self.ReceiveTick`
  (params (DeltaSeconds :type "Float (single-precision)"))
  (bind _as_bp_hero (`self.As BP Hero`))
  (`|ExecutionSequence`
    (:`then_1`
      ;[0.4497 0.0588 1 1 50] HitReaction Tick
      ;;[1 1 1] FinterpToZero
      (bind _output_get (set `self.HitReactionTimeRemaining` (- (`KismetMathLibrary.FInterpTo` (`self.HitReactionTimeRemaining`) 0.0 DeltaSeconds 5.0) (* DeltaSeconds 0.1))))
      (if (<= _output_get 0.01)
        ;;[1 1 1] STOP SIMULATION
        (set `self.HitReactionTimeRemaining` 0.0)
        (`self.ToggleSimulation` false)
        (`self.SetComponentTickEnabled` false)
        (`|ExecutionSequence`)
        (else
          ;;[0.1785 0.1427 1 1 31] HitTime > 0
          (`SkeletalMeshComponent.SetAllBodiesBelowPhysicsBlendWeight` (`self.Mesh`) (`self.UpperBodyBone`) (* (`KismetMathLibrary.FMin` (`self.HitReactionTimeRemaining`) 1.0) 1.0) false true)
          ;;;[1 1 1] STUMBLE
          (`ALSBaseCharacter.SetRotationMode` _as_bp_hero "LookingDirection" true)
          (`Pawn.AddMovementInput` _as_bp_hero (* (`KismetMathLibrary.Normal` (`self.LastImpulse`)) 0.1) 1.0 false))))))

(fn `BreakHitResult`
  (params (Hit :type "HitResult Structure (by ref)"))
  (returns (Location :type "Vector Structure") (HitBoneName :type Name) (Impulse :type "Vector Structure") (ImpactPoint :type "Vector Structure") (ImpactNormal :type "Vector Structure") (bInitialOverlap :type Boolean))
  (bind (_bblockinghit _binitialoverlap _time _distance _location _impactpoint _normal _impactnormal _physmat _hitactor _hitcomponent _hitbonename _bonename _hititem _elementindex _faceindex _tracestart _traceend) (`GameplayStatics.BreakHitResult` Hit))
  (bind _impulsestrength (`self.ImpulseStrength`))
  ;[1 1 1] SET IMPULSE
  (return _location _hitbonename (* (* (`KismetMathLibrary.Normal` _impactnormal) (`KismetMathLibrary.MakeVector` _impulsestrength _impulsestrength)) -1.0) _impactpoint _impactnormal _binitialoverlap))

(fn `DEBUG_Impulse`
  (bind _hitlocation (`self.HitLocation`))
  (`KismetSystemLibrary.DrawDebugArrow` _hitlocation (+ _hitlocation (`self.LastImpulse`)) 1.0 (struct) 1.0))

(fn `InitFunction`
  ;[1 1 1] Set References
  (bind _asbp_hero (cast `/Game/BP_Hero` (`self.GetOwner`)))
  (set `self.As BP Hero` _asbp_hero)
  (set `self.Mesh` (`Character.Mesh` (`self.As BP Hero`)))
  (set `self.Character Movement` (`Character.CharacterMovement` (`self.As BP Hero`)))
  ;[1 1 1] Init Physical Component
  (bind _returnvalue (`|AddComponentByClass` (`self.As BP Hero`) "/Script/Engine.PhysicalAnimationComponent"))
  (bind _output_get (set `self.PhysicalAnimComponent` _returnvalue))
  (`PhysicalAnimationComponent.SetSkeletalMeshComponent` _output_get (`self.Mesh`))
  (`SkeletalMeshComponent.SetAllBodiesBelowSimulatePhysics` (`self.Mesh`) (`self.UpperBodyBone`) false true)
  (`SkeletalMeshComponent.SetAllBodiesBelowPhysicsBlendWeight` (`self.Mesh`) (`self.UpperBodyBone`) 0.0 false true))

(fn `OnRagdollChangeState`
  (params (isRagdoll :type Boolean))
  ;[1 1 1] Delegate in BP_Hero
  (if isRagdoll
    (`PhysicalAnimationComponent.ApplyPhysicalAnimationProfileBelow` (`self.PhysicalAnimComponent`) "root" "None" true true)
    (set `self.HitReactionTimeRemaining` 0.0)
    (`KismetSystemLibrary.PrintString` "RAGDOLL START")
    (else
      (set `self.HitReactionTimeRemaining` 0.0)
      (`KismetSystemLibrary.PrintString` "RAGDOLL END"))))

(fn `ResetAnimationProfile`
  (`|ExecutionSequence`
    (:`then_0`
      (`PhysicalAnimationComponent.ApplyPhysicalAnimationProfileBelow` (`self.PhysicalAnimComponent`) "Thigh_L" "Strong" true false)
      (`PhysicalAnimationComponent.ApplyPhysicalAnimationProfileBelow` (`self.PhysicalAnimComponent`) "Thigh_R" "Strong" true false)
      (`PhysicalAnimationComponent.ApplyPhysicalAnimationProfileBelow` (`self.PhysicalAnimComponent`) (`self.UpperBodyBone`) "Strong" true false)
      (`PhysicalAnimationComponent.SetStrengthMultiplyer` (`self.PhysicalAnimComponent`) 1.0)
      (`SkeletalMeshComponent.SetAllBodiesBelowPhysicsBlendWeight` (`self.Mesh`) "Pelvis" (`self.BlendWeightDefault`) true true))
    (:`then_1`
      (`SkeletalMeshComponent.SetAllBodiesBelowPhysicsBlendWeight` (`self.Mesh`) "Thigh_L" 10.0 false true)
      (`SkeletalMeshComponent.SetAllBodiesBelowPhysicsBlendWeight` (`self.Mesh`) "Thigh_R" 10.0 false true))))

(fn `ToggleSimulation`
  (params (simulate :type Boolean))
  ;[1 1 1] != RAGDOLL CHECK
  (if (`|EnumInequality` (`ALSBaseCharacter.MovementState` (`self.As BP Hero`)) "Ragdoll")
    ;[1 1 1] SET VARIABLE
    (set `self.isSimulating` simulate)
    (`self.ResetAnimationProfile`)
    (`|ExecutionSequence`
      (:`then_0`
        ;[1 1 1] Turn Simulation OFF (Pelvis )
        (`SkeletalMeshComponent.SetAllBodiesBelowSimulatePhysics` (`self.Mesh`) "Pelvis" false true))
      (:`then_1`
        ;[1 1 1] Turn Simulation ON/OFF (UPPER BODY )
        (`SkeletalMeshComponent.SetAllBodiesBelowSimulatePhysics` (`self.Mesh`) (`self.UpperBodyBone`) (`self.isSimulating`) true))
      (:`then_2`
        ;[1 1 1] Turn Simulation ON/OFF (LOWER BODY )
        (`SkeletalMeshComponent.SetAllBodiesBelowSimulatePhysics` (`self.Mesh`) "Thigh_L" (`self.isSimulating`) true)
        (`SkeletalMeshComponent.SetAllBodiesBelowSimulatePhysics` (`self.Mesh`) "Thigh_R" (`self.isSimulating`) true))
      (:`then_3`
        ;[1 1 1] Enable Collision
        (`PrimitiveComponent.SetCollisionEnabled` (`self.Mesh`) (select `bool` (`self.isSimulating`) :`false` "QueryOnly" :`true` "QueryAndPhysics" :!type "ECollisionEnabled Enum")))
      (:`then_6`
        ;[1 0.9259 0.1099 1 30] ENABLE?DISABLE TICK
        (`self.SetComponentTickEnabled` (`self.isSimulating`)))
      (:`then_7`
        ;[0.2862 0 1 1 44] END
        (return)))
    (else
      (set `self.isSimulating` false))))

(fn `TriggerRagdollEnd`
  (`ALSBaseCharacter.RagdollEnd` (`self.As BP Hero`)))

(fn `TriggerRagdollStart`
  (`ALSBaseCharacter.RagdollStart` (`self.As BP Hero`)))

(fn `TurnRagdollFor`
  (params (Time :type "Float (single-precision)"))
  (`self.TriggerRagdollStart`)
  (`KismetSystemLibrary.K2_SetTimer` null "TriggerRagdollEnd" Time))